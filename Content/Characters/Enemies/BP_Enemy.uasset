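; BP_Enemy is an enemy driven by the BT_Zombie behavior tree, with a health bar widget.
; On BeginPlay it passes itself to the WBP_EnemyHealth widget as its Enemy reference.
; When possessed, it waits briefly, runs the tree on its AIController, then stores the first player's character under the Player blackboard key.
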(event `self.ReceiveBeginPlay`
  (bind _aswbp_enemy_health (cast `/Game/UI/WBP_EnemyHealth` (`WidgetComponent.GetUserWidgetObject` (`self.Health Bar`))))
  (set `/Game/UI/WBP_EnemyHealth.Enemy` self _aswbp_enemy_health))

(event `self.ReceivePossessed`
  (params (NewController :type "Controller Object Reference"))
  (`KismetSystemLibrary.Delay` 0.2)
  (bind _asaicontroller (cast `AIController` NewController))
  (bind _returnvalue (`AIController.RunBehaviorTree` _asaicontroller "/Game/Characters/Enemies/BT_Zombie.BT_Zombie"))
  (if _returnvalue
    (bind _output_get (set `self.Player` (cast `PlayerCharacter` (`GameplayStatics.GetPlayerCharacter` 0) :!pure true)))
    (`BlackboardComponent.SetValueAsObject` (`AIController.Blackboard` _asaicontroller) "Player" _output_get)))

(fn `UserConstructionScript`)